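; BP_FiringComponent is a weapon component that fires projectiles from its own world transform.
; TryFire spawns the Projectile class only if it derives from BallProjectile, passing the owner as Owner and, cast to Pawn, as Instigator.
; If Weapon also derives from GunActor, it plays a fire sound and reports a noise event at that location.
; An IsChild helper gates both steps through class-hierarchy checks.
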(fn `Try Fire`
  (bind _returnvalue (`self.K2_GetComponentToWorld`))
  (bind _returnvalue_2 (`self.GetOwner`))
  (bind _projectile (`self.Projectile`))
  (bind _location (.location _returnvalue))
  (bind _aspawn (cast `Pawn` _returnvalue_2 :!pure true))
  (`self.IsChild` _projectile "/Script/TestingGround.BallProjectile"
    (:`true`
      (`|SpawnActorFromClass` _projectile _returnvalue "AdjustIfPossibleButAlwaysSpawn" "OverrideRootScale" _returnvalue_2 _aspawn)
      (`self.IsChild` (`self.Weapon`) "/Script/TestingGround.GunActor"
        (:`true`
          (`GameplayStatics.SpawnSoundAtLocation` "/Game/Characters/Audio/WeaponFire02.WeaponFire02" _location (struct) 1.0 1.0 0.0 null null)
          (`AISense_Hearing.ReportNoiseEvent` _location 1.0 _aspawn))))))