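; Laser projectile Blueprint that deals point damage to whatever it hits.
; Each hit applies BaseDamage along the hit normal, with the projectile itself as damage causer.
; On a bounce, it stops simulating only if the struck actor's AI controller matches EnemyController.
; The movement component's stop event then destroys the projectile.
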(event `self.ReceiveHit`
  (params (MyComp :type "PrimitiveComponent Object Reference") (Other :type "Actor Object Reference") (OtherComp :type "PrimitiveComponent Object Reference") (bSelfMoved :type Boolean) (HitLocation :type "Vector Structure") (HitNormal :type "Vector Structure") (NormalImpulse :type "Vector Structure") (Hit :type "HitResult Structure (by ref)"))
  (`GameplayStatics.ApplyPointDamage` Other (`self.Base Damage`) HitNormal Hit null self))

(event `self.ProjectileMovement.OnProjectileBounce`
  (params (ImpactResult :type "HitResult Structure (by ref)") (ImpactVelocity :type "Vector Structure (by ref)"))
  (if (== (`AIBlueprintHelperLibrary.GetAIController` (`.HitActor` (`GameplayStatics.BreakHitResult` ImpactResult))) "/Game/Characters/AI/EnemyController.EnemyController")
    (`ProjectileMovementComponent.StopSimulating` (`self.ProjectileMovement`) ImpactResult)))

(event `self.ProjectileMovement.OnProjectileStop`
  (params (ImpactResult :type "HitResult Structure (by ref)"))
  (`self.K2_DestroyActor`))

(fn `UserConstructionScript`)