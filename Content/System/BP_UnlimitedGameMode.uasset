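; BP_UnlimitedGameMode is a game mode that builds a chain of tiles, one per SpawnNextTile call.
; Each call spawns TileToSpawn at NextTileTransform, adjusting for collision but always spawning, and passes NavPool to the new tile.
; The tile's attach location then becomes the transform for the next spawn.
; BeginPlay only calls its parent, so tile spawning is triggered from outside this graph.
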(event `self.SpawnNextTile`
  (bind _returnvalue (`|SpawnActorFromClass` (`self.TileToSpawn`) (`self.NextTileTransform`) "AdjustIfPossibleButAlwaysSpawn" "OverrideRootScale" null null))
  (`Tile.SetPool` _returnvalue (`self.NavPool`))
  (bind _returnvalue_2 (`Tile.GetAttachLocation` _returnvalue))
  (set `self.NextTileTransform` _returnvalue_2))

(event `self.ReceiveBeginPlay`
  (`parent.ReceiveBeginPlay`))

(fn `UserConstructionScript`
  (`parent.UserConstructionScript`))