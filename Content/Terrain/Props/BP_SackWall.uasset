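; BP_SackWall procedurally builds a stepped sack wall at BeginPlay from Height, Width and Angle.
; EachRow stacks centred rows upward, each one sack shorter than the row below.
; EachSack adds static mesh components along each row, stepping yaw and a sine-based X offset to bend the wall across Angle.
; A single-sack row spawns a separate BP_Sack actor instead of a mesh component.
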(event `self.ReceiveBeginPlay`
  (`self.Each Row`))

(fn `Calc Angle Delta`
  (returns (`Angle Differential` :type "Float (double-precision)"))
  (return (/ (`self.Angle`) (`KismetMathLibrary.Conv_IntToDouble` (+ (`self.Height`) (`self.Width`) -2)))))

(fn `Each Row`
  (locals (`Vertical Start` :type "Float (double-precision)") (`Horizontal Start` :type "Float (double-precision)") (`Start Angle` :type "Float (double-precision)") (`Object Count` :type Integer))
  (for _index (range (`self.Height`))
    (bind _returnvalue (- (+ (`self.Height`) (`self.Width`)) (+ _index 1)))
    (`self.Each Sack` (* _index 30.0) (+ (* -90 (/ (`KismetMathLibrary.Conv_IntToDouble` _returnvalue) 2.0)) 45.0) (+ (/ (`self.Angle`) -2.0) (* (`KismetMathLibrary.Conv_IntToDouble` _index) (`self.Calc Angle Delta`) 0.5)) _returnvalue)))

(fn `Each Sack`
  (params (`Vert Start` :type "Float (double-precision)") (`Hor Start` :type "Float (double-precision)") (`Ang Start` :type "Float (double-precision)") (`Object Count` :type Integer))
  (locals (Vert :type "Float (double-precision)") (Hor :type "Float (double-precision)") (Ang :type "Float (double-precision)") (Dep :type "Float (double-precision)"))
  (bind _hor (`local.Hor`))
  (bind _ang (`local.Ang`))
  (set `local.Vert` `Vert Start`)
  (set `local.Hor` `Hor Start`)
  (set `local.Dep` `Hor Start`)
  (set `local.Ang` `Ang Start`)
  (if (== `Object Count` 1)
    (`|SpawnActorFromClass` "/Game/Terrain/Props/BP_Sack.BP_Sack_C" (`KismetMathLibrary.MakeTransform` (+ (`self.K2_GetActorLocation`) (`KismetMathLibrary.MakeVector` 0.0 0.0 (`local.Vert`)))) "Undefined" "OverrideRootScale" self null)
    (else
      (for _ (range 1 (+ `Object Count` 1))
        (`AddComponent|NODE_AddStaticMeshComponent-0` :`RelativeTransform` (`KismetMathLibrary.MakeTransform` (`KismetMathLibrary.MakeVector` (* (`KismetMathLibrary.DegSin` _ang) _hor -0.5) _hor (`local.Vert`)) (`KismetMathLibrary.MakeRotator` 0.0 0.0 _ang)))
        (set `local.Hor` (+ _hor 90.0))
        (set `local.Dep` (+ (`local.Dep`) (* (`KismetMathLibrary.DegCos` (`self.Calc Angle Delta`)) 90.0)))
        (set `local.Ang` (+ _ang (`self.Calc Angle Delta`)))))))

(fn `UserConstructionScript`
  (locals (SackVert :type "Float (double-precision)") (SackHor :type "Float (double-precision)") (SackCount :type Integer)))