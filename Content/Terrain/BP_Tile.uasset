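; BP_Tile is a terrain tile that spawns its own grass, props, rocks and enemy characters on BeginPlay.
; A generated spawn parameter list feeds PlaceActors to populate the tile.
; Its gate starts locked and red, turning passable and green while the player overlaps DetectionField.
; An Arrow supplies the attach transform with unit scale, and player overlap with GCField destroys the tile.
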(event `self.ReceiveBeginPlay`
  (`self.Lock Gate` true)
  (`GrassComponent.SpawnGrass` (`self.Grass1`))
  (`GrassComponent.SpawnGrass` (`self.Grass2`))
  (`GrassComponent.SpawnGrass` (`self.Grass3`))
  (`self.Actor Spawning`))

(event `self.Detection Field.OnComponentBeginOverlap`
  (params (OverlappedComponent :type "PrimitiveComponent Object Reference") (OtherActor :type "Actor Object Reference") (OtherComp :type "PrimitiveComponent Object Reference") (OtherBodyIndex :type Integer) (bFromSweep :type Boolean) (SweepResult :type "HitResult Structure (by ref)"))
  (`self.Is Player Actor` OtherActor)
  (`self.Lock Gate` false))

(event `self.Detection Field.OnComponentEndOverlap`
  (params (OverlappedComponent :type "PrimitiveComponent Object Reference") (OtherActor :type "Actor Object Reference") (OtherComp :type "PrimitiveComponent Object Reference") (OtherBodyIndex :type Integer))
  (`self.Is Player Actor` OtherActor)
  (`self.Lock Gate` true))

(event `self.GC Field.OnComponentBeginOverlap`
  (params (OverlappedComponent :type "PrimitiveComponent Object Reference") (OtherActor :type "Actor Object Reference") (OtherComp :type "PrimitiveComponent Object Reference") (OtherBodyIndex :type Integer) (bFromSweep :type Boolean) (SweepResult :type "HitResult Structure (by ref)"))
  (`self.Is Player Actor` OtherActor)
  (`self.K2_DestroyActor`))

(fn `Actor Spawning`
  (locals (`To Spawn` :type "Array of  Structure"))
  (`self.PlaceActors` (`self.Generate Spawn Parameters`)))

(fn `Generate Spawn Parameters`
  (returns (NewParam :type "Array of SpawnParameters Structure"))
  (return (`|MakeArray` (make `SpawnParameters` "/Game/Terrain/Props/BP_Container.BP_Container_C" (`|MakeArray` "None" :!type "Name") 0 4 0.25 4.0 false) (make `SpawnParameters` "/Game/Terrain/Props/BP_Rock_01.BP_Rock_01_C" (`|MakeArray` "None" :!type "Name") 0 4 0.25 4.0 true false) (make `SpawnParameters` "/Game/Terrain/Props/BP_Rock_05.BP_Rock_05_C" (`|MakeArray` "None" :!type "Name") 0 4 0.25 4.0 true) (make `SpawnParameters` "/Game/Terrain/Props/BP_Rock_17.BP_Rock_17_C" (`|MakeArray` "None" :!type "Name") 0 4 0.25 4.0 true false) (make `SpawnParameters` "/Game/Terrain/Props/BP_Box.BP_Box_C" (`|MakeArray` "None" :!type "Name")) (make `SpawnParameters` "/Game/Terrain/Props/BP_Canister.BP_Canister_C" (`|MakeArray` "None" :!type "Name")) (make `SpawnParameters` "/Game/Terrain/Props/BP_SackWall.BP_SackWall_C" (`|MakeArray` "None" :!type "Name")) (make `SpawnParameters` "/Game/Characters/BP_Character.BP_Character_C" (`|MakeArray` "Enemy" :!type "Name") 3 7 0.25 4.0 false true true))))

(fn `GetAttachLocation`
  (returns (ReturnValue :type "Transform Structure"))
  (bind (_returnvalue_location _returnvalue_rotation) (`KismetMathLibrary.BreakTransform` (`SceneComponent.K2_GetComponentToWorld` (`self.Arrow`))))
  (return (`KismetMathLibrary.MakeTransform` _returnvalue_location _returnvalue_rotation)))

(fn `Lock Gate`
  (params (Lock :type Boolean))
  (bind _gate (`self.Gate`))
  (if Lock
    (`PrimitiveComponent.SetCollisionEnabled` _gate "QueryAndPhysics")
    (`PrimitiveComponent.SetMaterial` _gate 0 "/Game/Terrain/MI_Barrier_Red.MI_Barrier_Red")
    (else
      (`PrimitiveComponent.SetCollisionEnabled` _gate "NoCollision")
      (`PrimitiveComponent.SetMaterial` _gate 0 "/Game/Terrain/MI_Barrier_Green.MI_Barrier_Green"))))

(fn `UserConstructionScript`)