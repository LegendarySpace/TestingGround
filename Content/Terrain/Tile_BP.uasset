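; Terrain tile Blueprint with a barrier gate and an attach point for positioning another piece.
; The gate starts locked on BeginPlay, and DetectionField overlaps pass through a player check to unlock it on entry and relock it on exit.
; LockGate toggles the gate's collision and swaps its red or green barrier material.
; GetAttachLocation returns the Arrow's world location with zero rotation and unit scale.
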(event `self.ReceiveBeginPlay`
  (`self.Lock Gate` true))

(event `self.Detection Field.OnComponentBeginOverlap`
  (params (OverlappedComponent :type "PrimitiveComponent Object Reference") (OtherActor :type "Actor Object Reference") (OtherComp :type "PrimitiveComponent Object Reference") (OtherBodyIndex :type Integer) (bFromSweep :type Boolean) (SweepResult :type "HitResult Structure (by ref)"))
  (`self.Is Player Actor` OtherActor)
  (`self.Lock Gate` false))

(event `self.Detection Field.OnComponentEndOverlap`
  (params (OverlappedComponent :type "PrimitiveComponent Object Reference") (OtherActor :type "Actor Object Reference") (OtherComp :type "PrimitiveComponent Object Reference") (OtherBodyIndex :type Integer))
  (`self.Is Player Actor` OtherActor)
  (`self.Lock Gate` true))

(fn `Get Attach Location`
  (returns (`Attach Transform` :type "Transform Structure"))
  (bind _returnvalue (`SceneComponent.K2_GetComponentToWorld` (`self.Arrow`)))
  (return (`KismetMathLibrary.MakeTransform` (`KismetMathLibrary.MakeVector` (.x (.location _returnvalue)) (.y (.location _returnvalue)) (.z (.location _returnvalue))))))

(fn `Lock Gate`
  (params (Lock :type Boolean))
  (bind _gate (`self.Gate`))
  (if Lock
    (`PrimitiveComponent.SetCollisionEnabled` _gate "QueryAndPhysics")
    (`PrimitiveComponent.SetMaterial` _gate 0 "/Game/Terrain/RedBarrier.RedBarrier")
    (else
      (`PrimitiveComponent.SetCollisionEnabled` _gate "NoCollision")
      (`PrimitiveComponent.SetMaterial` _gate 0 "/Game/Terrain/GreenBarrier.GreenBarrier"))))

(fn `UserConstructionScript`)